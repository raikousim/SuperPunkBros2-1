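; Camera actor that follows the player pawn along X in one direction, using a dead zone.
; BeginPlay snaps it to the pawn's X and offset Z while keeping its own Y, then stores that location.
; Each Tick, pawn movement beyond the forward threshold pushes the stored X by the overshoot and pins Z to a hardcoded height.
; The actor then moves to the stored location, so it never tracks backward.
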(event `self.ReceiveBeginPlay`
  (bind (_returnvalue _x _y _z) (`self.ActorLocation`))
  (`self.K2_SetActorLocation` (`KismetMathLibrary.MakeVector` _x (.y (`self.K2_GetActorLocation`)) _z))
  (set `self.CameraLocation` (`self.K2_GetActorLocation`)))

(event `self.ReceiveTick`
  (params (DeltaSeconds :type "Float (single-precision)"))
  (`|ExecutionSequence`
    (:`then_0`
      (if (> (`.X` (`self.ActorLocation`)) (`self.Camera Deadzone`))
        (bind _returnvalue (`self.Move Dead Zone`))
        (set `self.CameraLocation` _returnvalue)))
    (:`then_1`
      (`self.K2_SetActorLocation` (`self.CameraLocation`)))))

(fn `ActorLocation`
  (returns (ReturnValue :type "Vector Structure") (X :type "Float (double-precision)") (Y :type "Float (double-precision)") (Z :type "Float (double-precision)"))
  (locals (NewLocalVar_0 :type "Vector Structure" :default (0.0 0.0 0.0)))
  (bind (_returnvalue_x _returnvalue_y _returnvalue_z) (`KismetMathLibrary.BreakVector` (`self.K2_GetActorLocation` (`Controller.K2_GetPawn` (`GameplayStatics.GetPlayerController` 0)))))
  (return (0.0 0.0 0.0) _returnvalue_x _returnvalue_y (+ _returnvalue_z (`self.PlayerZ`))))

(fn `Camera Deadzone`
  (returns (X :type "Float (double-precision)"))
  (return (+ (.x (`self.K2_GetActorLocation`)) (`self.Deadzone`))))

(fn `Move Dead Zone`
  (returns (ReturnValue :type "Vector Structure"))
  (return (`KismetMathLibrary.MakeVector` (+ (- (`.X` (`self.ActorLocation`)) (`self.Camera Deadzone`)) (.x (`self.CameraLocation`))) (.y (`self.CameraLocation`)) -630.0)))

(fn `UserConstructionScript`)