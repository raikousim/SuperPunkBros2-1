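; CollisionCamera is an actor that moves with the player and toggles its own collision based on what overlaps it.
; Each tick it takes X from the CameraDead actor minus the BoxZ offset, and Y and Z from the player's pawn.
; When its Trigger begins an overlap, it enables actor collision for the player character and disables it for any other actor.
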(event `self.ReceiveTick`
  (params (DeltaSeconds :type "Float (single-precision)"))
  (`self.K2_SetActorLocation` (`KismetMathLibrary.MakeVector` (- (.x (`self.K2_GetActorLocation` (`self.CameraDead`))) (`self.BoxZ`)) (.y (`self.K2_GetActorLocation` (`Controller.K2_GetPawn` (`GameplayStatics.GetPlayerController` 0)))) (.z (`self.K2_GetActorLocation` (`Controller.K2_GetPawn` (`GameplayStatics.GetPlayerController` 0)))))))

(event `self.Trigger.OnComponentBeginOverlap`
  (params (OverlappedComponent :type "PrimitiveComponent Object Reference") (OtherActor :type "Actor Object Reference") (OtherComp :type "PrimitiveComponent Object Reference") (OtherBodyIndex :type Integer) (bFromSweep :type Boolean) (SweepResult :type "HitResult Structure (by ref)"))
  (if (== OtherActor (`GameplayStatics.GetPlayerCharacter` 0))
    (`self.SetActorEnableCollision` true)
    (else
      (`self.SetActorEnableCollision` false))))

(fn `UserConstructionScript`)