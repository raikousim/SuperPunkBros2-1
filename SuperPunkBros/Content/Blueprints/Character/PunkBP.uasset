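; PunkBP is the player character of a Mario-style side-scroller, with single-axis movement, sprint and variable-height jump.
; Releasing jump can reset upward velocity to a fixed value, depending on jump count, height and vertical speed.
; BeginPlay caches the first brick, mushroom (Champi) and Goomba actors found.
; Tick polls them: mushroom Eat shows Grand and enlarges the capsule once, while Goomba Attack toggles KillShape visibility.
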(event `self.ReceiveBeginPlay`
  ;[1 1 1] Cast Actors
  (`self.AddBriqueVariable`)
  (`self.GetChampiVariable`)
  (`self.GetGoombaVariable`))

(event `InputAxis|MoveRight`
  (params (AxisValue :type "Float (single-precision)"))
  ;[1 1 1] Basics Movements
  (`self.AddMovementInput` (-1.0 0.0 0.0) AxisValue))

(event `InputAction|Sprint`
  (params (Key :type "Key Structure"))
  (bind _charactermovement (`self.CharacterMovement`))
  ;[1 1 1] Sprint
  (:`Pressed`
    (set `CharacterMovementComponent.MaxWalkSpeed` (`self.SprintSpeed`) _charactermovement))
  (:`Released`
    (set `CharacterMovementComponent.MaxWalkSpeed` (`self.WalkSpeed`) _charactermovement)))

(event `InputAction|InJump`
  (params (Key :type "Key Structure"))
  ;[1 1 1] Analog Jump
  (:`Pressed`
    (`self.StartJump`))
  (:`Released`
    (`self.StopJump`)))

(event `self.ReceiveTick`
  (params (DeltaSeconds :type "Float (single-precision)"))
  (`self.ChampiEffect`)
  (bind _asgoom_ba_bp (cast `/Game/Blueprints/Ennemy/GoomBaBP` (`self.GoombaBP`)))
  (if (`/Game/Blueprints/Ennemy/GoomBaBP.Attack?` _asgoom_ba_bp)
    (`SceneComponent.SetHiddenInGame` (`self.KillShape`) false false)
    (else
      (`SceneComponent.SetHiddenInGame` (`self.KillShape`) true false))))

(fn `AddBriqueVariable`
  (bind _outactors (`GameplayStatics.GetAllActorsOfClass` "/Game/Blueprints/Brique/BriqueBP.BriqueBP_C"))
  (set `self.brique` (`|GetArrayItem` _outactors)))

(fn `ChampiEffect`
  (bind _aschampi_bp (cast `/Game/Blueprints/Brique/ChampiBP` (`self.ChampiBP`)))
  (if (`/Game/Blueprints/Brique/ChampiBP.Eat?` _aschampi_bp)
    (`SceneComponent.SetHiddenInGame` (`self.Grand`) false false)
    (`self.GrewUp`)
    (else
      (`SceneComponent.SetHiddenInGame` (`self.Grand`) true false))))

(fn `GetChampiVariable`
  (bind _outactors (`GameplayStatics.GetAllActorsOfClass` "/Game/Blueprints/Brique/ChampiBP.ChampiBP_C"))
  (set `self.ChampiBP` (`|GetArrayItem` _outactors)))

(fn `GetGoombaVariable`
  (bind _outactors (`GameplayStatics.GetAllActorsOfClass` "/Game/Blueprints/Ennemy/GoomBaBP.GoomBaBP_C"))
  (set `self.GoombaBP` (`|GetArrayItem` _outactors)))

(fn `GetNewHeight`
  (returns (ReturnValue :type "Float (double-precision)"))
  (return (* (`CapsuleComponent.GetScaledCapsuleHalfHeight` (`self.CapsuleComponent`)) 2.0)))

(fn `GetNewLoc`
  (returns (ReturnValue :type "Vector Structure"))
  (bind (_returnvalue_x _returnvalue_y _returnvalue_z) (`KismetMathLibrary.BreakVector` (`self.K2_GetActorLocation` (`Controller.K2_GetPawn` (`GameplayStatics.GetPlayerController` 0)))))
  (return (`KismetMathLibrary.MakeVector` _returnvalue_x _returnvalue_y (+ _returnvalue_z 25.0))))

(fn `GetSceneLoc`
  (returns (ReturnValue :type "Vector Structure"))
  (return (`self.K2_GetActorLocation` (`ActorComponent.GetOwner` (`self.Scene`)))))

(fn `GrewUp`
  (if (not (`self.Is>0?`))
    (`self.K2_SetActorLocation` (`self.GetNewLoc`))
    (`CapsuleComponent.SetCapsuleHalfHeight` (`self.CapsuleComponent`) (`self.GetNewHeight`) true)))

(fn `Is>0?`
  (returns (ReturnValue :type Boolean))
  (bind _output_get (set `self.SetNumber` (+ (`self.SetNumber`) 1.0)))
  (return (> _output_get 1.0)))

(fn `StartJump`
  (`self.Jump`)
  (set `self.NbJump` (+ (`self.NbJump`) 1.0))
  (if (not (`NavMovementComponent.IsFalling` (`self.CharacterMovement`)))
    (set `self.NbJump` 0.0)))

(fn `StopJump`
  (bind _returnvalue_x (`KismetMathLibrary.BreakVector` (`self.GetVelocity` (`GameplayStatics.GetPlayerCharacter` 0))))
  (if (> (`self.NbJump`) 0.0)
    _
    (elif (> (.z (`self.K2_GetActorLocation`)) (`self.MaxHigh`))
      _
      (elif (not (< (.z (`MovementComponent.Velocity` (`self.CharacterMovement`))) 0.0))
        (set `MovementComponent.Velocity` (`KismetMathLibrary.MakeVector` _returnvalue_x 0.0 300.0) (`self.CharacterMovement`))))))

(fn `UserConstructionScript`)