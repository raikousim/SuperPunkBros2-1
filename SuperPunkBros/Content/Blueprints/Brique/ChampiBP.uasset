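; Mario-style mushroom pickup character tied to the first special brick found in the level.
; Each tick it stays hidden without collision while that brick's Hide flag is set, then appears and walks along +X.
; If its velocity is zero after a short delay, it latches Stop and walks along -X from then on.
; Player overlap sets Eat, hides it and disables collision; jump and destroy helpers are not called here.
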(event `self.ReceiveBeginPlay`
  (`self.GetSpecialBriqueBP`)
  (`self.GetPunkVariable`))

(event `self.ReceiveTick`
  (params (DeltaSeconds :type "Float (single-precision)"))
  (if (`self.Stop?`)
    (`self.AddMovementInput` (-1.0 0.0 0.0))
    (else
      (bind _hide_ (`self.SearchHide`))
      (if _hide_
        (`self.MakeChampiDontMove`)
        (else
          (`self.MakeChampiMove`)
          (`KismetSystemLibrary.Delay` 0.2)
          (if (`self.Velocity0?`)
            (set `self.Stop?` true)))))))

(event `self.Box.OnComponentBeginOverlap`
  (params (OverlappedComponent :type "PrimitiveComponent Object Reference") (OtherActor :type "Actor Object Reference") (OtherComp :type "PrimitiveComponent Object Reference") (OtherBodyIndex :type Integer) (bFromSweep :type Boolean) (SweepResult :type "HitResult Structure (by ref)"))
  (if (== OtherActor (`GameplayStatics.GetPlayerCharacter` 0))
    (set `self.Eat?` true)
    (`SceneComponent.SetHiddenInGame` (`self.Champi`) true false)
    (`self.SetActorEnableCollision` false)))

(fn `AddBriqueVariable`
  (bind _outactors (`GameplayStatics.GetAllActorsOfClass` "/Game/Blueprints/Brique/BriqueBP.BriqueBP_C"))
  (set `self.brique` (`|GetArrayItem` _outactors)))

(fn `DestroyChampi`
  (params (A :type "Object Object Reference"))
  (if (== A (`GameplayStatics.GetPlayerCharacter` 0))
    (`self.K2_DestroyActor`)))

(fn `GetPunkVariable`
  (bind _outactors (`GameplayStatics.GetAllActorsOfClass` "/Game/Blueprints/Character/PunkBP.PunkBP_C"))
  (set `self.punkBP` (`|GetArrayItem` _outactors)))

(fn `GetSpecialBriqueBP`
  (bind _outactors (`GameplayStatics.GetAllActorsOfClass` "/Game/Blueprints/Brique/SpecialbriqueBP.SpecialbriqueBP_C"))
  (set `self.SpecialBrique` (`|GetArrayItem` _outactors)))

(fn `MakeChampiDontMove`
  (`SceneComponent.SetHiddenInGame` (`self.Champi`) true false)
  (`self.SetActorEnableCollision` false))

(fn `MakeChampiMove`
  (`SceneComponent.SetHiddenInGame` (`self.Champi`) false false)
  (`self.SetActorEnableCollision` true)
  (`self.AddMovementInput` (1.0 0.0 0.0)))

(fn `SearchHide`
  (returns (`Hide?` :type Boolean))
  (bind _asspecialbrique_bp (cast `/Game/Blueprints/Brique/SpecialbriqueBP` (`self.SpecialBrique`)))
  (return (`/Game/Blueprints/Brique/SpecialbriqueBP.Hide?` _asspecialbrique_bp)))

(fn `StartJump`
  (`self.Jump`))

(fn `StopJump`
  (bind _returnvalue_x (`KismetMathLibrary.BreakVector` (`self.GetVelocity` (`GameplayStatics.GetPlayerCharacter` 0))))
  (if (> 0.0 0.0)
    _
    (elif (> (.z (`self.K2_GetActorLocation`)) 0.0)
      _
      (elif (not (< (.z (`MovementComponent.Velocity` (`self.CharacterMovement`))) 0.0))
        (set `MovementComponent.Velocity` (`KismetMathLibrary.MakeVector` _returnvalue_x 0.0 300.0) (`self.CharacterMovement`))))))

(fn `UserConstructionScript`)

(fn `Velocity0?`
  (returns (ReturnValue :type Boolean))
  (return (== (`self.GetVelocity`) (0.0 0.0 0.0))))