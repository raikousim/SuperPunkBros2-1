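; BriqueBP is a brick actor that bumps when the player character overlaps its Box.
; The overlap calls Move, which moves the Brique component to a location raised by NewZ, then after a short delay to one lowered by NewZ.
; GetNewLoc and GetOldLoc derive both targets from the actor's world location, though MoveComponentTo takes them as relative locations.
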(event `self.Box.OnComponentBeginOverlap`
  (params (OverlappedComponent :type "PrimitiveComponent Object Reference") (OtherActor :type "Actor Object Reference") (OtherComp :type "PrimitiveComponent Object Reference") (OtherBodyIndex :type Integer) (bFromSweep :type Boolean) (SweepResult :type "HitResult Structure (by ref)"))
  (if (== OtherActor (`GameplayStatics.GetPlayerCharacter` 0))
    (`|ExecutionSequence`
      (:`then_0`
        (`KismetSystemLibrary.MoveComponentTo` (`self.Brique`) (`self.GetNewLoc`)))
      (:`then_1`
        (`KismetSystemLibrary.Delay` 0.2)
        (`KismetSystemLibrary.MoveComponentTo` (`self.Brique`) (`self.GetOldLoc`))))))

(fn `GetNewLoc`
  (returns (ReturnValue :type "Vector Structure"))
  (return (`KismetMathLibrary.MakeVector` (.x (`self.K2_GetActorLocation`)) (.y (`self.K2_GetActorLocation`)) (+ (.z (`self.K2_GetActorLocation`)) (`self.NewZ`)))))

(fn `GetOldLoc`
  (returns (ReturnValue :type "Vector Structure"))
  (return (`KismetMathLibrary.MakeVector` (.x (`self.K2_GetActorLocation`)) (.y (`self.K2_GetActorLocation`)) (- (.z (`self.K2_GetActorLocation`)) (`self.NewZ`)))))

(fn `UserConstructionScript`)